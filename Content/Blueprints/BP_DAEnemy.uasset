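; BP_DAEnemy is an enemy Blueprint that carries a mutant claw weapon and reacts to nearby players.
; On BeginPlay it spawns BP_MutantClawWeapon, snaps it to the mesh's left hand socket, disables its collision and sets itself as owner.
; A Sphere component acts as the detection zone, calling NoticePlayer when a DAPlayer begins overlapping and LosePlayer when one leaves.
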(event `self.ReceiveBeginPlay`
  (bind _returnvalue (`|SpawnActorFromClass` "/Game/Blueprints/BP_MutantClawWeapon.BP_MutantClawWeapon_C" (`KismetMathLibrary.MakeTransform` (0.0 0.0 0.0)) "AlwaysSpawn" "OverrideRootScale"))
  (bind _output_get (set `self.Weapon` _returnvalue))
  (`self.K2_AttachToComponent` _output_get (`self.Mesh`) "LeftHandSocket" "SnapToTarget" "SnapToTarget" "SnapToTarget" true)
  (`DAWeaponBase.DisableCollision` _output_get)
  (set `DAWeaponBase.DAOwner` self _output_get))

(event `self.Sphere.OnComponentBeginOverlap`
  (params (OverlappedComponent :type "PrimitiveComponent Object Reference") (OtherActor :type "Actor Object Reference") (OtherComp :type "PrimitiveComponent Object Reference") (OtherBodyIndex :type Integer) (bFromSweep :type Boolean) (SweepResult :type "HitResult Structure (by ref)"))
  (bind _asdaplayer (cast `DAPlayer` OtherActor))
  (`self.NoticePlayer` _asdaplayer))

(event `self.Sphere.OnComponentEndOverlap`
  (params (OverlappedComponent :type "PrimitiveComponent Object Reference") (OtherActor :type "Actor Object Reference") (OtherComp :type "PrimitiveComponent Object Reference") (OtherBodyIndex :type Integer))
  (bind _asdaplayer (cast `DAPlayer` OtherActor))
  (`self.LosePlayer` _asdaplayer))

(fn `UserConstructionScript`)