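; Mutant claw weapon that damages a player when its box collision overlaps them.
; Overlaps count only for components tagged Character on a DAPlayer actor.
; Damage comes from GetCurrentDamage using the owner's and target's attributes, then goes to the player's GetHit.
; Collision is disabled right after a successful hit.
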(event `self.Box.OnComponentBeginOverlap`
  (params (OverlappedComponent :type "PrimitiveComponent Object Reference") (OtherActor :type "Actor Object Reference") (OtherComp :type "PrimitiveComponent Object Reference") (OtherBodyIndex :type Integer) (bFromSweep :type Boolean) (SweepResult :type "HitResult Structure (by ref)"))
  (if (`ActorComponent.ComponentHasTag` OtherComp "Character")
    (bind _asdaplayer (cast `DAPlayer` OtherActor))
    (`DACharacter.GetHit` _asdaplayer (`self.GetCurrentDamage` (`DACharacter.GetAttributes` (`self.DAOwner`)) (`DACharacter.GetAttributes` _asdaplayer)))
    (`self.DisableCollision`)))

(fn `UserConstructionScript`
  (`parent.UserConstructionScript`))