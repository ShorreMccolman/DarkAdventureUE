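; BP_HealConsumable is a consumable that heals its owning character gradually over its duration.
; On activation it computes a per-tick increment from potency, duration and time step.
; Each timer event applies that increment through the owner's HealCharacter call.
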(event `self.OnActivate`
  (set `self.Increment` (* (/ (`self.Potency`) (`self.Duration`)) (`self.TimeStep`))))

(event `self.OnTimer`
  (`DACharacter.HealCharacter` (`self.DAOwner`) (`self.Increment`)))

(fn `UserConstructionScript`
  (`parent.UserConstructionScript`))